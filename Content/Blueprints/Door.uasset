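; Door Blueprint that swings open and closed when interacted with while something overlaps its Box trigger.
; Box begin and end overlaps set an interactable flag, with no filter on the overlapping actor, which gates OnInteract.
; DoorInteraction toggles the open state and plays or reverses the DoorAnimation timeline, whose DoorMovement track drives the Scene component's relative yaw through a quarter turn.
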(event OnComponentBeginOverlap(Box)
  (params (OverlappedComponent :type Primitive%20Component%20Object%20Reference) (OtherActor :type Actor%20Object%20Reference) (OtherComp :type Primitive%20Component%20Object%20Reference) (OtherBodyIndex :type Integer) (bFromSweep :type Boolean) (SweepResult :type Hit%20Result%20Structure%20%28by%20ref%29))
  (Variables|Default|SetisInteractable true))

(event OnComponentEndOverlap(Box)
  (params (OverlappedComponent :type Primitive%20Component%20Object%20Reference) (OtherActor :type Actor%20Object%20Reference) (OtherComp :type Primitive%20Component%20Object%20Reference) (OtherBodyIndex :type Integer))
  (Variables|Default|SetisInteractable false))

(event Custom|DoorInteraction
  (if (Variables|Default|GetisDoorOpen)
    (Variables|Default|SetisDoorOpen false)
    (bind _doormovement (Timeline|DoorAnimation Reverse)
      (:Update
        (Transformation|SetRelativeRotation (Variables|Default|GetScene) (Math|Rotator|MakeRotator 0.0 0.0 (* _doormovement -9e+01)) false false)))
    (else
      (Variables|Default|SetisDoorOpen true)
      (Timeline|DoorAnimation Play))))

(event EventBeginPlay
  (Variables|Default|SetisInteractable false)
  (Variables|Default|SetisDoorOpen false))

(event EventOnInteract
  (if (Variables|Default|GetisInteractable)
    (CallFunction|DoorInteraction)))

(fn ConstructionScript)