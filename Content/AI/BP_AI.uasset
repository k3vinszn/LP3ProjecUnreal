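; BP_AI is an AI-controlled pawn that reports to its Blackboard when it sees the player.
; Its PawnSensing sight event filters for BP_Character, then sets the HasSeenPlayer key through the AI controller's Blackboard.
; A retriggerable delay clears the key two seconds after the last sighting, so repeated sightings keep it true.
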(event OnSeePawn(PawnSensing)
  (params (Pawn :type Pawn%20Object%20Reference))
  (Utilities|Casting|CastToBP_Character Pawn)
  (AI|Components|Blackboard|SetValueasBool (AI|GetBlackboard (AI|GetAIController self)) (Utilities|Name|MakeLiteralName "HasSeenPlayer") true)
  (Utilities|FlowControl|RetriggerableDelay 2.0)
  (AI|Components|Blackboard|SetValueasBool (AI|GetBlackboard (AI|GetAIController self)) (Utilities|Name|MakeLiteralName "HasSeenPlayer") false))

(fn ConstructionScript)